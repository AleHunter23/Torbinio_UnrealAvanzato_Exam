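; Random pickup that alternates between the points and poison materials on looping, offset timers, disguising whether it helps or harms.
; When the player character overlaps, a coin flip picks one of two DT_Exam rows, applies its score to the point UI, then hides the pickup and disables its collision.
; If the total drops below zero, it disables input and calls PlayerDeath after a delay.
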(event Collision|EventActorBeginOverlap
  (params (OtherActor :type Actor%20Object%20Reference))
  (if (Math|Random|RandomBool)
    (bind _asbp_third_person_character (Utilities|Casting|CastToBP_ThirdPersonCharacter OtherActor))
    (bind _returnvalue (Utilities|GetDataTableRow "/Game/Exam_Level/DataTable/DT_Exam.DT_Exam" "AumentoB")
      (:then
        (Variables|Default|SetItemType (.itemtype _returnvalue))
        (Variables|Default|SetDescription (.description _returnvalue))
        (bind _output_get (Variables|Default|SetPunteggio (.punteggio _returnvalue)))
        (Default|PointChange (Variables|/Game/Exam_Level/BluePrints/BP_ThirdPersonCharacter.BP_ThirdPersonCharacter_C|GetPointUI _asbp_third_person_character) _output_get)
        (Rendering|SetVisibility (Variables|Default|GetPoints) false false)
        (Collision|SetCollisionEnabled (Variables|Default|GetSphere) "NoCollision")
        (if (< (Variables|/Game/Exam_Level/UI/WBP_ExamUI.WBP_ExamUI_C|GetPointAmount (Variables|/Game/Exam_Level/BluePrints/BP_ThirdPersonCharacter.BP_ThirdPersonCharacter_C|GetPointUI _asbp_third_person_character)) 0)
          (Development|PrintString "YOURE GOING TO DIE IN 3 SECONDS" true true "(R=1.000000,G=0.149234,B=0.143981,A=1.000000)")
          (Variables|/Game/Exam_Level/BluePrints/BP_ThirdPersonCharacter.BP_ThirdPersonCharacter_C|SetCanDie _asbp_third_person_character true)
          (Input|DisableInput _asbp_third_person_character (Game|GetPlayerController 0))
          (Utilities|FlowControl|Delay 3.0)
          (Default|PlayerDeath _asbp_third_person_character)
          (Development|PrintString "Deleted Save Files")
          (else
            (Development|PrintString "Point Collected" true true "(R=1.000000,G=0.853183,B=0.116600,A=1.000000)")))))
    (else
      (bind _asbp_third_person_character_2 (Utilities|Casting|CastToBP_ThirdPersonCharacter OtherActor))
      (bind _returnvalue_2 (Utilities|GetDataTableRow "/Game/Exam_Level/DataTable/DT_Exam.DT_Exam" "DiminuzioneB")
        (:then
          (Variables|Default|SetItemType (.itemtype _returnvalue_2))
          (Variables|Default|SetDescription (.description _returnvalue_2))
          (bind _output_get_2 (Variables|Default|SetPunteggio (.punteggio _returnvalue_2)))
          (Default|PointChange (Variables|/Game/Exam_Level/BluePrints/BP_ThirdPersonCharacter.BP_ThirdPersonCharacter_C|GetPointUI _asbp_third_person_character_2) _output_get_2)
          (Rendering|SetVisibility (Variables|Default|GetPoints) false false)
          (Collision|SetCollisionEnabled (Variables|Default|GetSphere) "NoCollision")
          (if (< (Variables|/Game/Exam_Level/UI/WBP_ExamUI.WBP_ExamUI_C|GetPointAmount (Variables|/Game/Exam_Level/BluePrints/BP_ThirdPersonCharacter.BP_ThirdPersonCharacter_C|GetPointUI _asbp_third_person_character_2)) 0)
            (Development|PrintString "YOURE GOING TO DIE IN 3 SECONDS" true true "(R=1.000000,G=0.149234,B=0.143981,A=1.000000)")
            (Variables|/Game/Exam_Level/BluePrints/BP_ThirdPersonCharacter.BP_ThirdPersonCharacter_C|SetCanDie _asbp_third_person_character_2 true)
            (Input|DisableInput _asbp_third_person_character_2 (Game|GetPlayerController 0))
            (Utilities|FlowControl|Delay 3.0)
            (Default|PlayerDeath _asbp_third_person_character_2)
            (Development|PrintString "Deleted Save Files")
            (else
              (Development|PrintString "Poison Collected" true true "(R=0.987438,G=0.079122,B=1.000000,A=1.000000)"))))))))

(event EventBeginPlay
  (Utilities|Time|SetTimerbyFunctionName 0 "Yellow" 0.4 true)
  (Utilities|FlowControl|Delay 0.2)
  (Utilities|Time|SetTimerbyFunctionName 0 "Purple" 0.4 true))

(fn ConstructionScript)

(fn Yellow
  (Rendering|Material|SetMaterial (Variables|Default|GetPoints) 0 "/Game/Exam_Level/Materials/MT_Points.MT_Points"))

(fn Purple
  (Rendering|Material|SetMaterial (Variables|Default|GetPoints) 0 "/Game/Exam_Level/Materials/MT_Poison.MT_Poison"))