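; BP_Points is a collectible pickup that awards score to BP_ThirdPersonCharacter on overlap.
; It reads its values from DT_Exam by RowName, sends Punteggio to the player's PointUI, then hides itself and disables its sphere collision.
; It also decrements the player's NumberofPoints counter.
; If none remain and the score is below MinimumRequired, it disables input and calls PlayerDeath after a short delay.
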(event Collision|EventActorBeginOverlap
  (params (OtherActor :type Actor%20Object%20Reference))
  (bind _asbp_third_person_character (Utilities|Casting|CastToBP_ThirdPersonCharacter OtherActor))
  (bind _returnvalue (Utilities|GetDataTableRow "/Game/Exam_Level/DataTable/DT_Exam.DT_Exam" (Variables|Default|GetRow%20Name))
    (:then
      (Variables|Default|SetItemType (.itemtype _returnvalue))
      (Variables|Default|SetDescription (.description _returnvalue))
      (bind _output_get (Variables|Default|SetPunteggio (.punteggio _returnvalue)))
      (Default|PointChange (Variables|/Game/Exam_Level/BluePrints/BP_ThirdPersonCharacter.BP_ThirdPersonCharacter_C|GetPointUI _asbp_third_person_character) _output_get)
      (Rendering|SetVisibility (Variables|Default|GetPoints) false false)
      (Collision|SetCollisionEnabled (Variables|Default|GetSphere) "NoCollision")
      (Variables|/Game/Exam_Level/BluePrints/BP_ThirdPersonCharacter.BP_ThirdPersonCharacter_C|SetNumberofPoints _asbp_third_person_character (- (Variables|/Game/Exam_Level/BluePrints/BP_ThirdPersonCharacter.BP_ThirdPersonCharacter_C|GetNumberofPoints _asbp_third_person_character) 1))
      (if (and (<= (Variables|/Game/Exam_Level/BluePrints/BP_ThirdPersonCharacter.BP_ThirdPersonCharacter_C|GetNumberofPoints _asbp_third_person_character) 0) (< (Variables|/Game/Exam_Level/UI/WBP_ExamLevel.WBP_ExamLevel_C|GetPointAmount (Variables|/Game/Exam_Level/BluePrints/BP_ThirdPersonCharacter.BP_ThirdPersonCharacter_C|GetPointUI _asbp_third_person_character)) (Variables|/Game/Exam_Level/BluePrints/BP_ThirdPersonCharacter.BP_ThirdPersonCharacter_C|GetMinimumRequired _asbp_third_person_character)))
        (Development|PrintString "YOURE GOING TO DIE IN 3 SECONDS" true true "(R=1.000000,G=0.149234,B=0.143981,A=1.000000)")
        (Variables|/Game/Exam_Level/BluePrints/BP_ThirdPersonCharacter.BP_ThirdPersonCharacter_C|SetCanDie _asbp_third_person_character true)
        (Input|DisableInput _asbp_third_person_character (Game|GetPlayerController 0))
        (Utilities|FlowControl|Delay 3.0)
        (Default|PlayerDeath _asbp_third_person_character)
        (Development|PrintString "Deleted Save Files")
        (else
          (Development|PrintString "Point Collected" true true "(R=1.000000,G=0.853183,B=0.116600,A=1.000000)"))))))

(fn ConstructionScript)