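; BP_Gate is a gate that opens into the exam level once the game mode's button counter equals two.
; OpenDoor checks that counter on BP_ThirdPersonGameMode, loads Exam_level as a level instance, then hides the Cube and disables its collision.
; CloseDoor restores the Cube's visibility and collision but leaves the loaded level in place.
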(event Custom|CloseDoor
  (Rendering|SetVisibility (Variables|Default|GetCube) true false)
  (Collision|SetCollisionEnabled (Variables|Default|GetCube) "QueryAndPhysics"))

(event Custom|OpenDoor
  (bind _asbp_third_person_game_mode (Utilities|Casting|CastToBP_ThirdPersonGameMode (Game|GetGameMode)))
  (if (== (Variables|/Game/ThirdPerson/Blueprints/BP_ThirdPersonGameMode.BP_ThirdPersonGameMode_C|GetButtonCounter _asbp_third_person_game_mode) 2)
    (Class|LevelStreamingDynamic|LoadLevelInstancebySoftObjectPtr "/Game/Exam_Level/Exam_level.Exam_level" "0, 0, 0" "0, 0, 0" "" 0 false)
    (Rendering|SetVisibility (Variables|Default|GetCube) false false)
    (Collision|SetCollisionEnabled (Variables|Default|GetCube) "NoCollision")))

(fn ConstructionScript)