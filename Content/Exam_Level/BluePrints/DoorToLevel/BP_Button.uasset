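; Interactable timed button that works with a second press to reach a shared count of two on BP_ThirdPersonGameMode.
; On interaction it increments ButtonCounter, latches Triggered, swaps its material and calls OpenDoor on its Pressed reference.
; After a configurable delay, if the count is not two, it undoes the increment, trigger and material, but not the OpenDoor call.
; CanInteract always returns false.
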(event EventOnInteraction
  (params (OtherActor :type BP%20Third%20Person%20Character%20Object%20Reference))
  (if (not (Variables|Default|GetTriggered))
    (bind _asbp_third_person_game_mode (Utilities|Casting|CastToBP_ThirdPersonGameMode (Game|GetGameMode)))
    (Variables|/Game/ThirdPerson/Blueprints/BP_ThirdPersonGameMode.BP_ThirdPersonGameMode_C|SetButtonCounter _asbp_third_person_game_mode (+ (Variables|/Game/ThirdPerson/Blueprints/BP_ThirdPersonGameMode.BP_ThirdPersonGameMode_C|GetButtonCounter _asbp_third_person_game_mode) 1))
    (Variables|Default|SetTriggered true)
    (Rendering|Material|SetMaterial (Variables|Default|GetButton) 0 "/Game/ThirdPerson/MI_ThirdPersonColWay.MI_ThirdPersonColWay")
    (Default|OpenDoor (Variables|Default|GetPressed))
    (Development|PrintString "TIMER PARTITO")
    (Utilities|FlowControl|Delay (Variables|Default|GetTime))
    (if (not (== (Variables|/Game/ThirdPerson/Blueprints/BP_ThirdPersonGameMode.BP_ThirdPersonGameMode_C|GetButtonCounter _asbp_third_person_game_mode) 2))
      (Variables|/Game/ThirdPerson/Blueprints/BP_ThirdPersonGameMode.BP_ThirdPersonGameMode_C|SetButtonCounter _asbp_third_person_game_mode (- (Variables|/Game/ThirdPerson/Blueprints/BP_ThirdPersonGameMode.BP_ThirdPersonGameMode_C|GetButtonCounter _asbp_third_person_game_mode) 1))
      (Variables|Default|SetTriggered false)
      (Rendering|Material|SetMaterial (Variables|Default|GetButton) 0 "/Game/Materials/MT_Enemies.MT_Enemies")
      (Development|PrintString "TOO SLOW!!!"))))

(fn ConstructionScript)

(fn CanInteract
  (return false))