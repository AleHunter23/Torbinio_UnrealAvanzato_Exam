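; BP_CUBESPIN rotates its Rotator component in quarter turns, apparently as a spinning cube or die.
; Four events, SpinForward, SpinBack, SpinRight and SpinLeft, each play a timeline that offsets roll or pitch from the stored Spinned rotation.
; On finish, each adds its 90-degree step to Spinned as separate Euler values.
; A CanSpin flag blocks new spins until the current one completes.
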(event Custom|SpinRight
  (if (Variables|Default|GetCanSpin)
    (Variables|Default|SetCanSpin false)
    (bind _left (Timeline|SpinningR PlayFromStart)
      (:Update
        (Transformation|SetRelativeRotation (Variables|Default|GetRotator) (Math|Rotator|MakeRotator (.roll (Variables|Default|GetSpinned)) (+ _left (.pitch (Variables|Default|GetSpinned))) (.yaw (Variables|Default|GetSpinned))) false false))
      (:Finished
        (Variables|Default|SetSpinned (Math|Rotator|MakeRotator (.roll (Variables|Default|GetSpinned)) (+ (.pitch (Variables|Default|GetSpinned)) 9e+01) (.yaw (Variables|Default|GetSpinned))))
        (Variables|Default|SetCanSpin true)))))

(event Custom|SpinBack
  (if (Variables|Default|GetCanSpin)
    (Variables|Default|SetCanSpin false)
    (bind _forward (Timeline|SpinningB PlayFromStart)
      (:Update
        (Transformation|SetRelativeRotation (Variables|Default|GetRotator) (Math|Rotator|MakeRotator (+ (* _forward -1.0) (.roll (Variables|Default|GetSpinned))) (.pitch (Variables|Default|GetSpinned)) (.yaw (Variables|Default|GetSpinned))) false false))
      (:Finished
        (Variables|Default|SetSpinned (Math|Rotator|MakeRotator (+ (.roll (Variables|Default|GetSpinned)) -9e+01) (.pitch (Variables|Default|GetSpinned)) (.yaw (Variables|Default|GetSpinned))))
        (Variables|Default|SetCanSpin true)))))

(event Custom|SpinLeft
  (if (Variables|Default|GetCanSpin)
    (Variables|Default|SetCanSpin false)
    (bind _left (Timeline|SpinningL PlayFromStart)
      (:Update
        (Transformation|SetRelativeRotation (Variables|Default|GetRotator) (Math|Rotator|MakeRotator (.roll (Variables|Default|GetSpinned)) (+ (* _left -1.0) (.pitch (Variables|Default|GetSpinned))) (.yaw (Variables|Default|GetSpinned))) false false))
      (:Finished
        (Variables|Default|SetSpinned (Math|Rotator|MakeRotator (.roll (Variables|Default|GetSpinned)) (+ (.pitch (Variables|Default|GetSpinned)) -9e+01) (.yaw (Variables|Default|GetSpinned))))
        (Variables|Default|SetCanSpin true)))))

(event Custom|SpinForward
  (if (Variables|Default|GetCanSpin)
    (Variables|Default|SetCanSpin false)
    (bind _forward (Timeline|SpinningF PlayFromStart)
      (:Update
        (Transformation|SetRelativeRotation (Variables|Default|GetRotator) (Math|Rotator|MakeRotator (+ _forward (.roll (Variables|Default|GetSpinned))) (.pitch (Variables|Default|GetSpinned)) (.yaw (Variables|Default|GetSpinned))) false false))
      (:Finished
        (Variables|Default|SetSpinned (Math|Rotator|MakeRotator (+ (.roll (Variables|Default|GetSpinned)) 9e+01) (.pitch (Variables|Default|GetSpinned)) (.yaw (Variables|Default|GetSpinned))))
        (Variables|Default|SetCanSpin true)))))

(fn ConstructionScript)